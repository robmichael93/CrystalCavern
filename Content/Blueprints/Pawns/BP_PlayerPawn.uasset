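; Player pawn that rolls via physics torque and restarts the level when it takes any damage.
; Move axis inputs apply acceleration-based torque to PlayerMesh, scaled by TorqueMultiplier.
; The camera fades in on BeginPlay; damage triggers a DoOnce-guarded Restart Level graph that fades out with audio, waits, then reopens the current level by name.
; Both fades and the reload delay share FadeOutDuration.
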(event EventBeginPlay
  ;[0.1661 0.9702 1] Game Start With Camera Fade In
  (CallFunction|CameraFadein))

(event Game|Damage|EventAnyDamage
  (params (Damage :type Float%20%28single-precision%29) (DamageType :type Damage%20Type%20Object%20Reference) (InstigatedBy :type Controller%20Object%20Reference) (DamageCauser :type Actor%20Object%20Reference))
  ;[0.7396 0.7396 0.7396] Restart Level After Damage
  (Utilities|RestartLevel))

(event Input|AxisEvents|InputAxisMoveForwards/Backwards
  (params (AxisValue :type Float%20%28single-precision%29))
  ;[1 0.4844 0.1146] Movement Functions for Player
  (CallFunction|MovePawnForwards/Backwards AxisValue))

(event Input|AxisEvents|InputAxisMoveLeft/Right
  (params (AxisValue :type Float%20%28single-precision%29))
  ;[1 0.4844 0.1146] Movement Functions for Player
  (CallFunction|MovePawnLeft/Right AxisValue))

(fn ConstructionScript)

(fn CameraFadein
  (CameraFades|StartCameraFade :self (Game|GetPlayerCameraManager 0) :FromAlpha 1.0 :Duration (Variables|Default|GetFadeOutDuration) :bHoldWhenFinished true))

(fn ReloadLevel
  (bind _returnvalue (Game|GetCurrentLevelName true))
  (Game|OpenLevel(byName) (Utilities|String|StringToName _returnvalue)))

(fn CameraFade
  (CameraFades|StartCameraFade :self (Game|GetPlayerCameraManager 0) :ToAlpha 1.0 :Duration (Variables|Default|GetFadeOutDuration) :bShouldFadeAudio true :bHoldWhenFinished true))

(fn MovePawnForwards/Backwards
  (params (A :type Float%20%28single-precision%29))
  (Class|PrimitiveComponent|AddTorqueinRadians (Variables|Default|GetPlayerMesh) (Math|Vector|MakeVector 0.0 (* A (Variables|Default|GetTorqueMultiplier)) 0.0) "None" true))

(fn MovePawnLeft/Right
  (params (A :type Float%20%28single-precision%29))
  (Class|PrimitiveComponent|AddTorqueinRadians (Variables|Default|GetPlayerMesh) (Math|Vector|MakeVector (* A (Variables|Default|GetTorqueMultiplier)) 0.0 0.0) "None" true))