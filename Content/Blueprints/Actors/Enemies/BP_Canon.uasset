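; BP_Canon is an enemy cannon that automatically fires projectiles in a repeating cycle from BeginPlay.
; After each FireRate delay, it spawns a BP_Projectile at ProjectileSpawnPoint's world location and rotation, scaled by ProjectileScale.
; CanonFireTimeline then animates the barrel along its relative Y axis, and its Canon Fired event track restarts the delay to sustain the loop.
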(event EventBeginPlay
  ;[0.1692 1 0.5832] Canon Firing
  (Utilities|FlowControl|Delay (Variables|ProjectileProperties|GetFireRate) :!label _label)
  (CallFunction|SpawnProjectile)
  (bind _canon_barrel_location (Timeline|Canon%20Fire%20Timeline PlayFromStart)
    (:Update
      (CallFunction|MoveCannonBarrel _canon_barrel_location))
    (:Canon%20Fired
      (goto _label))))

(fn ConstructionScript)

(fn SpawnProjectile
  (Game|SpawnActorfromClass "/Game/Blueprints/Actors/Projectiles/BP_Projectile.BP_Projectile_C" (Math|Transform|MakeTransform (Transformation|GetWorldLocation (Variables|Default|GetProjectile%20Spawn%20Point)) (Transformation|GetWorldRotation (Variables|Default|GetProjectile%20Spawn%20Point)) (Math|Conversions|ToVector(Float) (Variables|Default|GetProjectileScale))) "Undefined" 0 0))

(fn MoveCannonBarrel
  (params (Cannon%20Barrel%20Y%20Location :type Float%20%28single-precision%29))
  (Transformation|SetRelativeLocation (Variables|Default|GetCanonBarrel) (Math|Vector|MakeVector 0.0 Cannon%20Barrel%20Y%20Location 0.0) false false))